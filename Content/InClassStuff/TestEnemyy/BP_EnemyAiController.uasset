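; BP_EnemyAiController is an enemy AI controller that runs BT_EnemyTree on BeginPlay and reacts to pawns spotted by PawnSensing.
; A sighting calls SetCanSeePlayer, then again after a retriggerable delay of twice the sensing interval, with true both times.
; SetCanSeePlayer ignores both inputs, always setting the sight key true and writing no object to the target key, so sight is never cleared.
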(event OnSeePawn(PawnSensing)
  (params (Pawn :type Pawn%20Object%20Reference))
  (CallFunction|SetCanSeePlayer true Pawn)
  (Utilities|FlowControl|RetriggerableDelay (* (Variables|/Script/AIModule.PawnSensingComponent|GetSensingInterval (Variables|Default|GetPawnSensing)) 2.0))
  (CallFunction|SetCanSeePlayer true Pawn))

(event EventBeginPlay
  (AI|RunBehaviorTree "/Game/InClassStuff/TestEnemyy/BT_EnemyTree.BT_EnemyTree"))

(event EventTick
  (params (DeltaSeconds :type Float%20%28single-precision%29)))

(fn ConstructionScript)

(fn SetCanSeePlayer
  (params (CanSeePlayer :type Boolean) (Player :type Pawn%20Object%20Reference))
  (bind _blackboard (Variables|Default|GetBlackboard))
  (AI|Components|Blackboard|SetValueasBool _blackboard (Variables|Default|GetBBCanSeePlayer) true)
  (AI|Components|Blackboard|SetValueasObject _blackboard (Variables|Default|GetBBPlayerTarget) 0))