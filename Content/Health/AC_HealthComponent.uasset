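; Actor component that stores an owner's health within a configurable minimum and maximum range.
; BeginPlay calls Init, which sets the bounds and fills health to max.
; Damage, Heal and HealFull route through a clamped SetHealth, while getters expose raw health, normalized health (relative to max only) and a death check at zero or below.
; Tick holds only an unreachable Delay and has no effect.
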(event EventBeginPlay
  (CallFunction|Init (Variables|Default|GetHealthMin) (Variables|Default|GetHealthMax)))

(event EventTick
  (params (DeltaSeconds :type Float%20%28single-precision%29))
  (if (> 0 0)
    (Utilities|FlowControl|Delay 0.2)))

(fn Heal
  (params (HealAmount :type Float%20%28double-precision%29))
  (CallFunction|SetHealth (Math|Float|Clamp(Float) (+ HealAmount (Variables|Default|GetHealth)) (Variables|Default|GetHealthMin) (Variables|Default|GetHealthMax))))

(fn Damage
  (params (DamageAmount :type Float%20%28double-precision%29))
  (CallFunction|SetHealth (Math|Float|Clamp(Float) (- (Variables|Default|GetHealth) DamageAmount) (Variables|Default|GetHealthMin) (Variables|Default|GetHealthMax))))

(fn GetHealth
  (return (Variables|Default|GetHealth)))

(fn SetHealth
  (params (NewHealth :type Float%20%28double-precision%29))
  (Variables|Default|SetHealth (Math|Float|Clamp(Float) NewHealth (Variables|Default|GetHealthMin) (Variables|Default|GetHealthMax))))

(fn HealFull
  (CallFunction|SetHealth (Variables|Default|GetHealthMax)))

(fn IsDead
  (return (<= (CallFunction|GetHealth) 0.0)))

(fn GetNormalizedHealth
  (return (/ (Variables|Default|GetHealth) (Variables|Default|GetHealthMax))))

(fn Init
  (params (MinHealth :type Float%20%28double-precision%29) (MaxHealth :type Float%20%28double-precision%29))
  (Variables|Default|SetHealthMin MinHealth)
  (bind _output_get (Variables|Default|SetHealthMax MaxHealth))
  (CallFunction|SetHealth _output_get))